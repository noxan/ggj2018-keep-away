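; Player character for a multiplayer ball-shooting game, with a point light showing who holds the ball.
; Tick moves and turns the character along clamped movement input.
; Either fire axis past a threshold clears HasBall and calls a server event that spawns a BallProjectile.
; StartGame input, or this character's destruction, gives the ball to a random player from MainGameMode's list when nobody holds one.
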(event `self.ReceiveTick`
  (params (DeltaSeconds :type "Float (single-precision)"))
  (bind _returnvalue (`KismetMathLibrary.ClampVectorSize` (`KismetMathLibrary.MakeVector` (`self.GetInputAxisValue`) (`self.GetInputAxisValue`)) 0.0 1.0))
  ;[1 1 1] Input handling
  (`|ExecutionSequence`
    (:`then_0`
      (`SceneComponent.SetVisibility` (`self.PointLight`) (`self.HasBall`) false))
    (:`then_1`
      (`SceneComponent.K2_SetWorldRotation` (`self.RootComponent`) (`KismetMathLibrary.Conv_VectorToRotator` _returnvalue) false false)
      (`self.AddMovementInput` _returnvalue))))

(event `InputAxis|FireForward`
  (params (AxisValue :type "Float (single-precision)"))
  ;[1 1 1] Shoot input action
  (bind _returnvalue (`KismetMathLibrary.MakeVector` AxisValue (stale `InputAxis|FireRight` AxisValue)))
  (if (and (`self.HasBall`) (> (`KismetMathLibrary.VSizeSquared` _returnvalue) 0.5)) :!label _label
    (set `self.HasBall` false)
    (`self.ServerShootBall` _returnvalue (`self.K2_GetActorLocation`))))

(event `InputAxis|FireRight`
  (params (AxisValue :type "Float (single-precision)"))
  ;[1 1 1] Shoot input action
  (goto _label))

(event `ServerShootBall`
  (params (direction :type "Vector Structure") (location :type "Vector Structure"))
  (bind _returnvalue (`KismetMathLibrary.Conv_VectorToRotator` direction))
  (bind _returnvalue_2 (+ location (`KismetMathLibrary.GreaterGreater_VectorRotator` (`self.BallSpawnOffset`) _returnvalue)))
  ;[1 1 1] Handle ball shoot on server
  (`/Engine/EditorBlueprintResources/ActorMacros.Switch Has Authority`
    (:`Authority`
      (`KismetSystemLibrary.PrintString` "Fire")
      (set `self.HasBall` false)
      (`KismetSystemLibrary.DrawDebugLine` _returnvalue_2 location (struct :`R` 1.0 :`A` 1.0) 20.0 10.0)
      (`|SpawnActorFromClass` "/Game/Blueprints/BallProjectile.BallProjectile_C" (`KismetMathLibrary.MakeTransform` _returnvalue_2 _returnvalue) "AlwaysSpawn" "OverrideRootScale" null self))))

(event `self.ReceiveDestroyed`
  ;[1 1 1] Remove self from player list
  (bind _asmain_game_mode (cast `/Game/Blueprints/MainGameMode` (`GameplayStatics.GetGameMode`)))
  (bind _players (`/Game/Blueprints/MainGameMode.Players` _asmain_game_mode))
  (`KismetArrayLibrary.Array_RemoveItem` _players self)
  (bind _ballfound (`self.isBallPresent` _players))
  ;[1 1 1] Give random player a ball
  (if _ballfound
    _
    (elif (> (`KismetArrayLibrary.Array_Length` _players) 0)
      (`KismetArrayLibrary.Array_Shuffle` _players)
      (set `/Game/Blueprints/MainCharacter.HasBall` true (`|GetArrayItem` _players)))))

(event `InputAction|StartGame`
  (params (Key :type "Key Structure"))
  (:`Pressed`
    (`self.ServerDistributeBall`)))

(event `ServerDistributeBall`
  ;[1 1 1] Give random player a ball
  (`/Engine/EditorBlueprintResources/ActorMacros.Switch Has Authority`
    (:`Authority`
      (bind _asmain_game_mode (cast `/Game/Blueprints/MainGameMode` (`GameplayStatics.GetGameMode`)))
      (bind _players (`/Game/Blueprints/MainGameMode.Players` _asmain_game_mode))
      (bind _ballfound (`self.isBallPresent` _players))
      (if (not _ballfound)
        (`KismetArrayLibrary.Array_Shuffle` _players)
        (set `/Game/Blueprints/MainCharacter.HasBall` true (`|GetArrayItem` _players))))))

(fn `isBallPresent`
  (params (MainCharacters :type "Array of /Game/Blueprints/MainCharacter Object Reference"))
  (returns (BallFound :type Boolean))
  ;[1 1 1] Return false if no ball was found in players array
  (for _array_element MainCharacters
    (bind _hasball (`/Game/Blueprints/MainCharacter.HasBall` _array_element))
    (if _hasball
      (return _hasball)))
  (return false))

(fn `UserConstructionScript`)