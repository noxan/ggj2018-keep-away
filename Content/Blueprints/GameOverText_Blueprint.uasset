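; Replicated game-over text actor that shows its text render when the match is down to one player or none.
; On Tick, the server reads the Players list from MainGameMode and sets Gameover when one or fewer remain.
; The Gameover RepNotify toggles the text's visibility to match the flag, so clients see the change.
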(event `self.ReceiveTick`
  (params (DeltaSeconds :type "Float (single-precision)"))
  (`/Engine/EditorBlueprintResources/ActorMacros.Switch Has Authority`
    (:`Authority`
      (bind _asmain_game_mode (cast `/Game/Blueprints/MainGameMode` (`GameplayStatics.GetGameMode`)))
      (set `self.Gameover` (<= (`KismetArrayLibrary.Array_Length` (`/Game/Blueprints/MainGameMode.Players` _asmain_game_mode)) 1)))))

(fn `OnRep_Gameover`
  (`SceneComponent.SetVisibility` (`self.TextRender`) (`self.Gameover`) false))

(fn `UserConstructionScript`)